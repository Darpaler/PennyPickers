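; BP_CoinScore is an actor that keeps a coin score and shows it on a text render component.
; On BeginPlay it resets the score to zero and enables input from the first player controller.
; Each Space Bar press increments the score directly, and Tick rewrites the displayed text with the current value every frame.
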(event `self.ReceiveBeginPlay`
  (set `self.CoinScore` 0)
  (`self.EnableInput` (`GameplayStatics.GetPlayerController` 0)))

(event `Key|SpaceBar`
  (params (Key :type "Key Structure"))
  (:`Pressed`
    (`/Engine/EditorBlueprintResources/StandardMacros.IncrementInt` (`self.CoinScore`))))

(event `self.ReceiveTick`
  (params (DeltaSeconds :type "Float (single-precision)"))
  (`TextRenderComponent.K2_SetText` (`self.TextRender`) (`KismetTextLibrary.Conv_IntToText` (`self.CoinScore`))))

(fn `UserConstructionScript`)