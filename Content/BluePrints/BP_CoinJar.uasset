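; BP_CoinJar is a coin jar actor that grows with the coin score.
; Every Tick it reads the score from its CoinScore reference and compares it to the default jar size divided by the penny size.
; Above that threshold it sets a uniform actor scale of score times penny size; otherwise it leaves the scale untouched.
; BeginPlay, overlap and construction logic are empty.
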(event `self.ReceiveBeginPlay`)

(event `self.ReceiveTick`
  (params (DeltaSeconds :type "Float (single-precision)"))
  (if (not (<= (`KismetMathLibrary.Conv_IntToDouble` (`/Game/BluePrints/BP_CoinScore.CoinScore` (`self.CoinScore`))) (/ (`self.Defualt Jar Size`) (`self.Size Of Penny`))))
    (`self.SetActorScale3D` (* (`KismetMathLibrary.Conv_IntVectorToVector` (`KismetMathLibrary.Conv_IntToIntVector` (`/Game/BluePrints/BP_CoinScore.CoinScore` (`self.CoinScore`)))) (`self.Size Of Penny`)))))

(fn `UserConstructionScript`)