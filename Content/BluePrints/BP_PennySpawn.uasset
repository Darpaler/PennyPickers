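; BP_PennySpawn is a spawner actor that creates copies of its referenced Penny at random navigable points around itself.
; On BeginPlay it enables input from player controller 0 and copies its CoinScore onto that Penny.
; Each P key press picks a point within PennyDistance on the nav mesh, spawns an actor of Penny's class there and gives it the same CoinScore.
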(event `self.ReceiveBeginPlay`
  (`self.EnableInput` (`GameplayStatics.GetPlayerController` 0))
  (set `/Game/BluePrints/BP_Penny.CoinScore` (`self.CoinScore`) (`self.Penny`)))

(event `Key|P`
  (params (Key :type "Key Structure"))
  (:`Pressed`
    (bind _returnvalue (`|SpawnActorFromClass` (`GameplayStatics.GetObjectClass` (`self.Penny`)) (`KismetMathLibrary.Conv_VectorToTransform` (`NavigationSystemV1.K2_GetRandomLocationInNavigableRadius` (`self.K2_GetActorLocation`) (`self.PennyDistance`) (`self.NavData`) null)) "Undefined" "OverrideRootScale" null null))
    (set `/Game/BluePrints/BP_Penny.CoinScore` (`self.CoinScore`) _returnvalue)))

(fn `UserConstructionScript`)