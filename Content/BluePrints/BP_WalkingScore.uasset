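; BP_WalkingScore is an actor that scores walking as pennies earned, based on the fuel cost of driving the same distance.
; It enables input from the first player controller on BeginPlay.
; Pressing Space divides DistanceWalked by MilesPerGallon, multiplies by GasPrice, and stores the truncated cent value in PenniesEarned.
; The graph only reads DistanceWalked and does not update or display it.
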(event `self.ReceiveBeginPlay`
  (`self.EnableInput` (`GameplayStatics.GetPlayerController` 0)))

(event `Key|SpaceBar`
  (params (Key :type "Key Structure"))
  (:`Pressed`
    (set `self.PenniesEarned` (`KismetMathLibrary.FTrunc` (* 100 (* (/ (`self.DistanceWalked`) (`self.MilesPerGallon`)) (`self.GasPrice`)))))))

(fn `UserConstructionScript`)